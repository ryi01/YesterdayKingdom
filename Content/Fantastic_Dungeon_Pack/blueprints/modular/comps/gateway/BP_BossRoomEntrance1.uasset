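; BP_BossRoomEntrance1 is a boss room gateway whose door starts open and closes on request.
; BeginPlay binds CloseDoor to an OnCloseRequested dispatcher and sets the door mesh to the open height.
; CloseDoor plays a timeline that interpolates the door's relative Z from open to closed, leaving X and Y untouched.
; The graph has no logic to reopen the door.
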(event Custom|CloseDoor
  (bind _mod_gateway_door_01_med_01_door (Variables|Default|GetMOD_Gateway_Door_01_med_01_door))
  (bind _relativelocation (Variables|/Script/Engine.SceneComponent|GetRelativeLocation _mod_gateway_door_01_med_01_door))
  (bind _doorlocation (Timeline|Timeline Play)
    (:Update
      (Transformation|SetRelativeLocation (Variables|Default|GetMOD_Gateway_Door_01_med_01_door) (Math|Vector|MakeVector (.x _relativelocation) (.y _relativelocation) (.z (Math|Vector|Lerp(Vector) (Variables|Default|GetOpenLocation%20) (Variables|Default|GetCloseLocation) _doorlocation))) false false))))

(event EventBeginPlay
  (bind _mod_gateway_door_01_med_01_door (Variables|Default|GetMOD_Gateway_Door_01_med_01_door))
  (bind _relativelocation (Variables|/Script/Engine.SceneComponent|GetRelativeLocation _mod_gateway_door_01_med_01_door))
  (EventDispatchers|BindEventtoOnCloseRequested (delegate Custom|CloseDoor))
  (Transformation|SetRelativeLocation (Variables|Default|GetMOD_Gateway_Door_01_med_01_door) (Math|Vector|MakeVector (.x _relativelocation) (.y _relativelocation) (.z (Variables|Default|GetOpenLocation%20))) false false))

(event Collision|EventActorBeginOverlap
  (params (OtherActor :type Actor%20Object%20Reference)))

(event EventTick
  (params (DeltaSeconds :type Float%20%28single-precision%29)))

(fn ConstructionScript)